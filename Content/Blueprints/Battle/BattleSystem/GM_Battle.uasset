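; Battle game mode that runs turn-based combat between party and enemy units, ordered by their SPD stat.
; On BeginPlay it switches to the top-down camera, gathers both teams, fills the battle HUD and sorts turn order fastest first.
; A DoOnce-gated loop starts each unit's combat component turn, binds to its turn-ended event and wraps the index.
; Helper functions remove units from teams and print victory or defeat.
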(event `self.ReceiveBeginPlay`
  (bind _outactors (`GameplayStatics.GetAllActorsOfClass` "/Game/Blueprints/UnitBase.UnitBase_C"))
  (set `self.actorArray` _outactors)
  (bind _returnvalue (`GameplayStatics.GetActorOfClass` "/Game/Blueprints/Battle/BattleSystem/TopDownCam.TopDownCam_C"))
  (bind _output_get (set `self.mainBattleCam` _returnvalue))
  (`PlayerController.SetViewTargetWithBlend` (`GameplayStatics.GetPlayerController` 0) _output_get 0.0 "VTBlend_Linear" 0.0 false)
  (bind _outactors_2 (`GameplayStatics.GetAllActorsOfClass` "/Game/Blueprints/Battle/Party/PartyUnitBase.PartyUnitBase_C"))
  (set `self.partyTeam` _outactors_2)
  (bind _outactors_3 (`GameplayStatics.GetAllActorsOfClass` "/Game/Blueprints/Battle/Enemies/EnemyUnitBase.EnemyUnitBase_C"))
  (set `self.enemyTeam` _outactors_3)
  (`KismetSystemLibrary.Delay` 0.2)
  (bind _asbattle_player_controller (cast `/Game/Blueprints/Battle/BattleSystem/BattlePlayerController` (`GameplayStatics.GetPlayerController` 0)))
  (set `self.battleHUD` (`/Game/Blueprints/Battle/BattleSystem/BattlePlayerController.battleHUD` _asbattle_player_controller))
  (for _array_element (`self.partyTeam`)
    (`/Game/UI/Widgets/BattleHUD.addPartyUnitToHUD` (`self.battleHUD`) _array_element _array_element))
  (bind _turnorder (`self.sortTurnOrder`))
  (set `self.turnOrder` _turnorder)
  (`self.Start Turns`))

(event `NextTurn`
  (bind _combatcomponent (`/Game/Blueprints/UnitBase.CombatComponent` (`|GetArrayItem` (`self.turnOrder`) (`self.currentTurnIndex`))))
  (`|ExecutionSequence`
    (:`then_0`
      (goto _label :!via `Reset`))
    (:`then_1`
      (`self.Start Turns`))))

(event `Start Turns`
  (bind _combatcomponent (`/Game/Blueprints/UnitBase.CombatComponent` (`|GetArrayItem` (`self.turnOrder`) (`self.currentTurnIndex`))))
  (`/Engine/EditorBlueprintResources/StandardMacros.DoOnce` false :!label _label
    (:`Completed`
      (`/Game/Blueprints/Battle/BattleSystem/CombatComponent.startTurn` _combatcomponent)
      (add `/Game/Blueprints/Battle/BattleSystem/CombatComponent.turnEnded` _combatcomponent (`|CreateDelegate` :!event `NextTurn`))
      (if (== (`self.currentTurnIndex`) (- (`KismetArrayLibrary.Array_Length` (`self.turnOrder`)) 1))
        (set `self.currentTurnIndex` 0)
        (else
          (set `self.currentTurnIndex` (+ (`self.currentTurnIndex`) 1)))))))

(fn `endBattle`
  (if (> (`KismetArrayLibrary.Array_Length` (`self.partyTeam`)) 0)
    (if (not (> (`KismetArrayLibrary.Array_Length` (`self.enemyTeam`)) 0))
      (`KismetSystemLibrary.PrintString` "VICTORY"))
    (else
      (`KismetSystemLibrary.PrintString` "DEFEAT"))))

(fn `removeActorFromList`
  (params (`Unit Char` :type "/Game/Blueprints/UnitBase Object Reference"))
  (bind _asparty_unit_base (cast `/Game/Blueprints/Battle/Party/PartyUnitBase` `Unit Char`)
    (:`then`
      (`KismetArrayLibrary.Array_RemoveItem` (`self.partyTeam`) _asparty_unit_base))
    (:`CastFailed`
      (bind _asenemy_unit_base (cast `/Game/Blueprints/Battle/Enemies/EnemyUnitBase` `Unit Char`))
      (`KismetArrayLibrary.Array_RemoveItem` (`self.enemyTeam`) _asenemy_unit_base))))

(fn `sortTurnOrder`
  (returns (turnOrder :type "Array of /Game/Blueprints/UnitBase Object Reference"))
  (locals (speedArray :type "Array of Float (double-precision)") (sortedActors :type "Array of /Game/Blueprints/UnitBase Object Reference"))
  (bind _speedarray (`local.speedArray`))
  (bind _indexofmaxvalue (`KismetMathLibrary.MaxOfFloatArray` _speedarray))
  (for _array_element (`self.actorArray`)
    (bind _combatcomponent (`/Game/Blueprints/UnitBase.CombatComponent` _array_element))
    (`/Engine/EditorBlueprintResources/StandardMacros.IsValid` _combatcomponent
      (:`Is Valid`
        (`KismetArrayLibrary.Array_Add` (`local.speedArray`) (`KismetMathLibrary.Conv_IntToDouble` (`.SPD_23_2BBFF9DD456844CC74751DA4E4A5C3FA` (break `/Game/Blueprints/Battle/Data/StatTable` (`/Game/Blueprints/Battle/BattleSystem/CombatComponent.battleStats` _combatcomponent))))))
      (:`Is Not Valid`
        (`KismetSystemLibrary.PrintString` "COMBAT COMPONENTS FUCKED"))))
  (if (> (`KismetArrayLibrary.Array_Length` _speedarray) 0) :!label _label
    (`KismetArrayLibrary.Array_Add` (`local.sortedActors`) (`|GetArrayItem` (`self.actorArray`) _indexofmaxvalue))
    (`KismetArrayLibrary.Array_Remove` (`self.actorArray`) _indexofmaxvalue)
    (`KismetArrayLibrary.Array_Remove` (`local.speedArray`) _indexofmaxvalue)
    (goto _label)
    (else
      (return (`local.sortedActors`)))))

(fn `UserConstructionScript`)