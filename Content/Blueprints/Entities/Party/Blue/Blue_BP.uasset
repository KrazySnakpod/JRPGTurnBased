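; Blue party character Blueprint that drives a flipbook sprite from its movement.
; Each tick it switches the sprite between the walk and idle flipbooks based on whether velocity is non-zero.
; It also turns the controller's yaw to face left or right from the sign of X velocity, keeping the last facing when X velocity is zero.
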(event `self.ReceiveTick`
  (params (DeltaSeconds :type "Float (single-precision)"))
  (`self.UpdateAnimation`)
  (`self.UpdateDirection`))

(event `UpdateAnimation`
  ;[0.006995 0.006995 0.006995] Update Animation
  (`PaperFlipbookComponent.SetFlipbook` (`self.Sprite`) (select `bool` (> (`KismetMathLibrary.VSize` (`MovementComponent.Velocity` (`self.CharacterMovement`))) 0.0) :`false` "/Game/Assets/Party/Blue/Flipbooks/Blue_Idle.Blue_Idle" :`true` "/Game/Assets/Party/Blue/Flipbooks/Blue_Walk.Blue_Walk" :!type "PaperFlipbook Object Reference")))

(event `UpdateDirection`
  ;[0.006995 0.006995 0.006995] Update Direction
  (`/Engine/EditorBlueprintResources/StandardMacros.IsValid` (`self.GetController`)
    (:`Is Valid`
      (`/Engine/EditorBlueprintResources/StandardMacros.CompareFloat` (.x (`MovementComponent.Velocity` (`self.CharacterMovement`)))
        (:`>`
          (`Controller.SetControlRotation` (`self.GetController`) (`KismetMathLibrary.MakeRotator` 0.0)))
        (:`<`
          (`Controller.SetControlRotation` (`self.GetController`) (`KismetMathLibrary.MakeRotator` 0.0 0.0 180.0)))))))

(fn `UserConstructionScript`)